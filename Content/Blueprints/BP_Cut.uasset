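; BP_Cut is an actor that builds a cut line of configurable length out of small chunks when play begins.
; GenerateCut calls itself recursively, counting down CutLength to zero and thus producing one chunk more than that value.
; Each call adds a thin static mesh and a larger box component, evenly spaced along local Y by an incrementing counter, and prints a debug message.
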(event `self.ReceiveBeginPlay`
  (`self.Generate Cut` (`self.Cut Length`)))

(fn `Generate Cut`
  (params (Length :type Integer))
  (returns (Finished :type Boolean))
  (bind _output_get (set `self.LengthNum` (+ (`self.LengthNum`) 1)))
  (bind _returnvalue (* _output_get 2.5))
  (`AddComponent|NODE_AddStaticMeshComponent-0` :`self` self :`RelativeTransform` (`KismetMathLibrary.MakeTransform` (`KismetMathLibrary.MakeVector` 0.0 _returnvalue) (struct) (0.02 0.025 0.001)))
  (`AddComponent|NODE_AddBoxComponent-0` :`self` self :`RelativeTransform` (`KismetMathLibrary.MakeTransform` (`KismetMathLibrary.MakeVector` 0.0 _returnvalue) (struct) (0.03 0.0375 0.06)))
  (`KismetSystemLibrary.PrintText` "cut chunk completed")
  (if (> Length 0)
    (bind _finished (`self.Generate Cut` (- Length 1)))
    (return _finished)
    (else
      (return true))))

(fn `UserConstructionScript`)