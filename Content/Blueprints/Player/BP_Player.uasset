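; BP_Player is the player pawn for a tape-trail game, steered left and right while it moves forward automatically.
; Tick pushes TapeMesh along control yaw, applies turn input and lowers the spawn cooldown unless both turns are held.
; Holding click drains tape and spawns BP_Trail at the mesh when off cooldown, opening the main menu when tape runs out.
; It also sets up input mapping, the HUD and the pause menu.
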(event `self.ReceiveBeginPlay`
  ; Add mapping context and get reference to player controller
  (bind _asplayer_controller (cast `PlayerController` (`self.GetController`)))
  (set `self.PlayerController_Ref` _asplayer_controller)
  (bind _returnvalue (pcsubsystem `EnhancedInputLocalPlayerSubsystem` _asplayer_controller))
  (`/Engine/EditorBlueprintResources/StandardMacros.IsValid` _returnvalue
    (:`Is Valid`
      (`EnhancedInputSubsystemInterface.AddMappingContext` _returnvalue "/Game/Blueprints/Player/Inputs/IMC_Player.IMC_Player" 0 (struct))
      (bind _returnvalue_2 (`|CreateWidget` "/Game/UI/WB_HUD.WB_HUD_C"))
      (`UserWidget.AddToViewport` _returnvalue_2 0))))

(event `EnhancedInput|/Game/Blueprints/Player/Inputs/IA_Left`
  (params (ActionValue :type Boolean) (ElapsedSeconds :type "Float (double-precision)") (TriggeredSeconds :type "Float (double-precision)") (InputAction :type "InputAction Object Reference" :default "/Game/Blueprints/Player/Inputs/IA_Left.IA_Left"))
  ; Left and Right turning
  (:`Triggered`
    (set `self.TurningLeft` true)
    ; Set physical rotation speed
    (set `self.Rotate` -1.2)
    ; Aligns the mesh to face the same way
    (`SceneComponent.K2_AddWorldRotation` (`self.Tape Mesh`) (`KismetMathLibrary.MakeRotator` 0.0 0.0 -3.0) false false))
  (:`Completed`
    (set `self.TurningLeft` false)
    (set `self.Rotate` 0.0)))

(event `EnhancedInput|/Game/Blueprints/Player/Inputs/IA_Right`
  (params (ActionValue :type Boolean) (ElapsedSeconds :type "Float (double-precision)") (TriggeredSeconds :type "Float (double-precision)") (InputAction :type "InputAction Object Reference" :default "/Game/Blueprints/Player/Inputs/IA_Right.IA_Right"))
  ; Left and Right turning
  (:`Triggered`
    (set `self.TurningRight` true)
    ; Set physical rotation speed
    (set `self.Rotate` 1.2)
    ; Aligns the mesh to face the same way
    (`SceneComponent.K2_AddWorldRotation` (`self.Tape Mesh`) (`KismetMathLibrary.MakeRotator` 0.0 0.0 3.0) false false))
  (:`Completed`
    (set `self.TurningRight` false)
    (set `self.Rotate` 0.0)))

(event `self.ReceiveTick`
  (params (DeltaSeconds :type "Float (single-precision)"))
  (bind (_returnvalue_roll _returnvalue_pitch _returnvalue_yaw) (`KismetMathLibrary.BreakRotator` (`self.GetControlRotation`)))
  ; On tick
  ; Move forward
  (`SceneComponent.K2_AddRelativeLocation` (`self.Tape Mesh`) (`KismetMathLibrary.GetForwardVector` (`KismetMathLibrary.MakeRotator` 0.0 0.0 _returnvalue_yaw)) false false)
  ; If not turning both ways at the same time
  (if (`KismetMathLibrary.BooleanNAND` (`self.TurningLeft`) (`self.TurningRight`))
    ; Turns the player physically
    (`PlayerController.AddYawInput` (`self.PlayerController_Ref`) (`self.Rotate`))
    ; Lower tape cooldown
    (set `self.TapeCooldown` (- (`self.TapeCooldown`) 0.01))))

(event `EnhancedInput|/Game/Blueprints/Player/Inputs/IA_Pause`
  (params (ActionValue :type Boolean) (ElapsedSeconds :type "Float (double-precision)") (TriggeredSeconds :type "Float (double-precision)") (InputAction :type "InputAction Object Reference" :default "/Game/Blueprints/Player/Inputs/IA_Pause.IA_Pause"))
  (bind _returnvalue (`GameplayStatics.GetPlayerController` 0))
  ; On pause (escape key), create pause widget, set input mode to UI and pause the game
  (:`Completed`
    (bind _returnvalue_2 (`|CreateWidget` "/Game/UI/WB_PauseMenu.WB_PauseMenu_C"))
    (`UserWidget.AddToViewport` _returnvalue_2 0)
    (set `PlayerController.bShowMouseCursor` true _returnvalue)
    (`WidgetBlueprintLibrary.SetInputMode_UIOnlyEx` _returnvalue null)
    (`GameplayStatics.SetGamePaused` true)))

(event `EnhancedInput|/Game/Blueprints/Player/Inputs/IA_Click`
  (params (ActionValue :type Boolean) (ElapsedSeconds :type "Float (double-precision)") (TriggeredSeconds :type "Float (double-precision)") (InputAction :type "InputAction Object Reference" :default "/Game/Blueprints/Player/Inputs/IA_Click.IA_Click"))
  (:`Triggered`
    ; Set tape amount. If it has ran out, open main menu. If not, spawn tape
    (bind _output_get (set `self.TapeAmount` (- (`self.TapeAmount`) 0.15)))
    (if (<= _output_get 0.0)
      (`GameplayStatics.OpenLevel` "MainMenu_Level")
      (elif (<= (`self.TapeCooldown`) 0.0)
        (`|SpawnActorFromClass` "/Game/Blueprints/BP_Trail.BP_Trail_C" (`KismetMathLibrary.MakeTransform` (`SceneComponent.K2_GetComponentLocation` (`self.Tape Mesh`)) (`SceneComponent.K2_GetComponentRotation` (`self.Tape Mesh`))) "Undefined" "MultiplyWithRoot" null null)
        (set `self.TapeCooldown` 0.04))))
  (:`Started`
    (set `self.TapeTrailActive` true))
  (:`Completed`
    (set `self.TapeTrailActive` false)))

(fn `UserConstructionScript`)